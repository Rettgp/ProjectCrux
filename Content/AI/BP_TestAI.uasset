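; Test AI character that dual-wields axes and deals melee damage on auto-attack notifies.
; BeginPlay runs BT_TestAI and assigns a random numeric name on authority, then spawns and attaches an axe to each hand socket without an authority check.
; Each notify sphere-traces forward from the attacking side's axe socket and applies fixed damage to the first hit, with debug drawing.
; Naming, weapon spawning and hit detection are marked as test code.
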(event EventAutoAttackNotify
  (params (AttackInfo :type Auto%20Attack%20Info%20Structure))
  (bind _autoattackside (Utilities|Struct|BreakAutoAttackInfo AttackInfo))
  (bind _rightaxe (Variables|Default|GetRightAxe))
  (bind _leftaxe (Variables|Default|GetLeftAxe))
  (bind _returnvalue (Utilities|Select :Index _autoattackside :LEFT _leftaxe :RIGHT _rightaxe))
  (bind _returnvalue_2 (Class|CruxWeapon|PrimarySocketLocation _returnvalue))
  ;[1 1 1] Test sphere trace for hit detection MAKE ME BETTER
  (bind (_outhits _returnvalue_3) (Collision|MultiSphereTraceByChannel _returnvalue_2 (+ _returnvalue_2 (* (Transformation|GetActorForwardVector) 2e+02)) 75.0 "TraceTypeQuery3" false 0 "ForDuration" true "(R=1.000000,G=0.000000,B=0.000000,A=1.000000)" "(R=0.000000,G=1.000000,B=0.000000,A=1.000000)" 2.0))
  (if _returnvalue_3
    (Game|Damage|ApplyDamage (.HitActor (Collision|BreakHitResult (Utilities|Array|Get(acopy) _outhits))) 25.0 (Game|GetInstigatorController) self)))

(event EventBeginPlay
  (|CallParentFunction)
  (Utilities|FlowControl|Sequence
    (:then_0
      (Networking|SwitchHasAuthority
        (:Authority
          (AI|RunBehaviorTree (AI|GetAIController self) "/Game/AI/BT_TestAI.BT_TestAI"))))
    (:then_1
      ;[1 1 1] Setup Player Name. TEST CODE
      (if (Ability|HasAuthority)
        (Variables|Default|SetActorName (Utilities|String|ToString(Integer) (Math|Random|RandomInteger 255)))))
    (:then_2
      ;[1 1 1] TEST CODE - Spawn Weapons
      (bind _returnvalue (Game|SpawnActorfromClass "/Game/Blueprints/Weapons/BP_Axe.BP_Axe_C" (Math|Transform|MakeTransform "0, 0, 0") "AlwaysSpawn" 0 0))
      (bind _output_get (Variables|Default|SetRightAxe _returnvalue))
      (Transformation|AttachComponentToComponent _output_get (Variables|Character|GetMesh) "RightHandSocket" "KeepRelative" "KeepRelative" "KeepRelative" true)
      (bind _returnvalue_2 (Game|SpawnActorfromClass "/Game/Blueprints/Weapons/BP_Axe.BP_Axe_C" (Math|Transform|MakeTransform "0, 0, 0") "AlwaysSpawn" 0 0))
      (bind _output_get_2 (Variables|Default|SetLeftAxe _returnvalue_2))
      (Transformation|AttachComponentToComponent _output_get_2 (Variables|Character|GetMesh) "LeftHandSocket" "KeepRelative" "KeepRelative" "KeepRelative" true))))

(fn ConstructionScript)