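; Character Blueprint that handles movement lock during attacks, floating damage numbers and loot drops on death.
; Tick disables movement while an auto attack runs and restores walking otherwise.
; Health changes caused by a CruxCharacter under a player controller show a damage widget only to that instigator when locally controlled.
; Die, commented as server-only, spawns a loot actor per inventory item and scatters them with random horizontal impulses.
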(event Custom|OnHealthChanged_Event_0
  (params (HealthComp :type Crux%20Health%20Component%20Object%20Reference) (Health :type Float%20%28single-precision%29) (HealthDelta :type Float%20%28single-precision%29) (DamageType :type Damage%20Type%20Object%20Reference) (InstigatedBy :type Controller%20Object%20Reference) (DamageCause :type Actor%20Object%20Reference))
  ;[1 1 1] Take Damage
  (bind _asplayer_controller (Utilities|Casting|CastToPlayerController InstigatedBy))
  (Utilities|IsValid _asplayer_controller
    (:Is%20Valid
      (Utilities|Casting|CastToCruxCharacter DamageCause)
      (CallFunction|DamageText HealthDelta _asplayer_controller self false))))

(event Custom|DamageText
  (params (Damage :type Float%20%28single-precision%29) (Instigator :type Player%20Controller%20Object%20Reference) (Target :type Actor%20Object%20Reference) (IsCrit :type Boolean))
  ;[1 1 1] Display Damage Text
  (if (Utilities|IsValid Instigator)
    (if (Pawn|IsLocalPlayerController Instigator)
      (bind _returnvalue (UserInterface|CreateWidget "/Game/UI/WBP_FloatingDamage.WBP_FloatingDamage_C" Instigator Damage Target IsCrit))
      (UserInterface|Viewport|AddtoViewport _returnvalue 0))))

(event EventTick
  (params (DeltaSeconds :type Float%20%28single-precision%29))
  (bind _charactermovement (Variables|Character|GetCharacterMovement))
  ;[1 1 1] Disable movement input when attacking
  (if (Variables|Default|GetAutoAttackStarted)
    (Pawn|Components|CharacterMovement|DisableMovement _charactermovement)
    (else
      (Pawn|Components|CharacterMovement|SetMovementMode _charactermovement "MOVE_Walking" 0))))

(event EventBeginPlay
  ;[1 1 1] Take Damage
  (EventDispatchers|AssignOnHealthChanged (Variables|Default|GetHealthComp) (delegate Custom|OnHealthChanged_Event_0)))

(event EventDie
  ;[1 1 1] Spawn Loot Drops (SERVER ONLY)
  (for _array_element (Class|CruxInventory|GetItems (Variables|Default|GetInventory))
    (bind _returnvalue (Game|SpawnActorfromClass "/Game/Blueprints/Items/BP_LootItem.BP_LootItem_C" (Math|Transform|MakeTransform (Transformation|GetActorLocation) "0, 0, 0" "1.000000,1.000000,1.000000") "AlwaysSpawn" 0 _array_element 0))
    (Physics|AddImpulse (Variables|/Game/Blueprints/Items/BP_LootItem.BP_LootItem_C|GetStaticMesh _returnvalue) (* (* (Math|Random|RandomUnitVector) (Math|Vector|MakeVector 1.0 1.0 0.0)) 2.5e+02) "None" true)))

(fn ConstructionScript)