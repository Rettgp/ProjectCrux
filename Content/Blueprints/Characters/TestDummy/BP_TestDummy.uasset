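; BP_TestDummy is a test character that wires up health bar HUDs, targeting feedback and floating damage numbers.
; BeginPlay creates both bars for a player controller, binds health changes and gives the server a random test name.
; Targeting toggles the target bar with a debug sphere, while CruxCharacter damage spawns floating text for locally controlled instigators.
; Attack movement lock and sphere-trace hit detection are unconnected test code.
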(event Custom|OnHealthChanged_Event_0
  (params (HealthComp :type Crux%20Health%20Component%20Object%20Reference) (Health :type Float%20%28single-precision%29) (HealthDelta :type Float%20%28single-precision%29) (DamageType :type Damage%20Type%20Object%20Reference) (InstigatedBy :type Controller%20Object%20Reference) (DamageCause :type Actor%20Object%20Reference))
  ;[1 1 1] Take Damage
  (bind _asplayer_controller (Utilities|Casting|CastToPlayerController InstigatedBy))
  (Utilities|IsValid _asplayer_controller
    (:Is%20Valid
      (Utilities|Casting|CastToCruxCharacter DamageCause)
      (CallFunction|DamageText HealthDelta _asplayer_controller self false))))

(event Custom|DamageText
  (params (Damage :type Float%20%28single-precision%29) (Instigator :type Player%20Controller%20Object%20Reference) (Target :type Actor%20Object%20Reference) (IsCrit :type Boolean))
  ;[1 1 1] Display Damage Text
  (if (Utilities|IsValid Instigator)
    (if (Pawn|IsLocalPlayerController Instigator)
      (bind _returnvalue (UserInterface|CreateWidget "/Game/UI/WBP_FloatingDamage.WBP_FloatingDamage_C" Instigator Damage Target IsCrit))
      (UserInterface|Viewport|AddtoViewport _returnvalue 0))))

(event EventTargeted
  (params (target :type Crux%20Character%20Object%20Reference))
  (bind _targethealthbar (Variables|Default|GetTargetHealthBar))
  (bind _targethealthbar_2 (Variables|Default|GetTargetHealthBar))
  (bind _returnvalue (Widget|IsVisible _targethealthbar))
  ;[1 1 1] On target selected/deselected update HUD
  (bind _output_get (Variables|/Game/UI/WBP_TargetHealthBar.WBP_TargetHealthBar_C|SetTargetActor (Variables|Default|GetTargetHealthBar) target))
  (if (Utilities|IsValid _output_get)
    (Rendering|Debug|DrawDebugSphere (Transformation|GetActorLocation _output_get) 64.0 12 "(R=1.000000,G=0.000000,B=0.014468,A=1.000000)" 1.0)
    (if (not _returnvalue)
      (UserInterface|Viewport|AddtoViewport _targethealthbar_2 0))
    (elif _returnvalue
      (Widget|RemovefromParent _targethealthbar_2))))

(event EventBeginPlay
  (bind _self self)
  (Utilities|FlowControl|Sequence
    (:then_0
      ;[1 1 1] Add Player and Target HUDs
      (bind _asplayer_controller (Utilities|Casting|CastToPlayerController (Pawn|GetController _self)))
      (bind _returnvalue (UserInterface|CreateWidget "/Game/UI/WBP_CharacterHealthBar.WBP_CharacterHealthBar_C" _asplayer_controller _self))
      (UserInterface|Viewport|AddtoViewport _returnvalue 0)
      (bind _returnvalue_2 (UserInterface|CreateWidget "/Game/UI/WBP_TargetHealthBar.WBP_TargetHealthBar_C" _asplayer_controller 0))
      (Variables|Default|SetTargetHealthBar _returnvalue_2))
    (:then_1
      ;[1 1 1] Take Damage
      (EventDispatchers|AssignOnHealthChanged (Variables|Default|GetHealthComp) (delegate Custom|OnHealthChanged_Event_0)))
    (:then_2
      ;[1 1 1] Setup Player Name. TEST CODE
      (if (Ability|HasAuthority)
        (Variables|Default|SetActorName (Utilities|String|ToString(Integer) (Math|Random|RandomInteger 255)))))))

(fn ConstructionScript)