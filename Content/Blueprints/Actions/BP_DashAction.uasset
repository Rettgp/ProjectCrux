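; BP_DashAction is an action that dashes its owner along the direction it faces.
; On Run, it casts the owner's movement component to CruxCharacterMovementComponent and calls Dash with the forward vector scaled by Velocity.
; On completion, it stops the character's movement immediately, then performs a movement component cast whose result is unused.
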(event EventOnCompleted
  (bind _actionowner (Variables|Default|GetActionOwner))
  (bind _charactermovement (Variables|/Script/Engine.Character|GetCharacterMovement _actionowner))
  (|CallParentFunction)
  (Components|Movement|StopMovementImmediately _charactermovement)
  (Utilities|Casting|CastToCruxCharacterMovementComponent _charactermovement))

(event EventRun
  (params (Owner :type Crux%20Character%20Object%20Reference))
  (|CallParentFunction Owner)
  (bind _ascrux_character_movement_component (Utilities|Casting|CastToCruxCharacterMovementComponent (Pawn|GetMovementComponent Owner)))
  (Class|CruxCharacterMovementComponent|Dash _ascrux_character_movement_component (* (Transformation|GetActorForwardVector Owner) (Variables|Default|GetVelocity))))