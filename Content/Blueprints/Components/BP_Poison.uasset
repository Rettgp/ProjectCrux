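; Poison status effect component that deals damage over time to the character that owns it.
; On begin play it attaches a scaled-up StatusEffectFx emitter to the character's particle system component, and destroys it on end play.
; Each EffectTick applies Damage to the owner with Instigator as causer, also passing the instigator's controller when it is a Pawn.
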(event EventEndPlay
  (params (EndPlayReason :type EEndPlayReason%20Enum :default "Destroyed"))
  (bind _spawnedparticle (Variables|Default|GetSpawnedParticle))
  (Utilities|IsValid _spawnedparticle
    (:Is%20Valid
      (Components|DestroyComponent _spawnedparticle))))

(event EventBeginPlay
  (bind _asbp_character (Utilities|Casting|CastToBP_Character (Components|GetOwner)))
  (bind _returnvalue (Effects|SpawnEmitterAttached (Variables|Default|GetStatusEffectFx) (Actor|GetComponentbyClass _asbp_character "/Script/Engine.ParticleSystemComponent") "None" "0, 0, 0" "0, 0, 0" "2.000000,2.000000,2.000000" "SnapToTargetIncludingScale"))
  (Variables|Default|SetSpawnedParticle _returnvalue))

(event EventEffectTick
  (bind _returnvalue (Components|GetOwner))
  (Utilities|IsValid (Components|GetOwner)
    (:Is%20Valid
      (bind _aspawn (Utilities|Casting|CastToPawn (Variables|Default|GetInstigator))
        (:then
          (Game|Damage|ApplyDamage _returnvalue (Variables|Default|GetDamage) (Pawn|GetController _aspawn) (Variables|Default|GetInstigator)))
        (:CastFailed
          (Game|Damage|ApplyDamage _returnvalue (Variables|Default|GetDamage) 0 (Variables|Default|GetInstigator)))))))